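; Zombie enemy actor that chases the first-person player and dies from a single projectile hit.
; A Box overlap sets the player as target and flags detection on ZombieAnimBP.
; While alive, Tick moves and turns it toward the target with fixed-alpha lerps, without sweep or navigation, so pursuit is frame-rate dependent.
; A projectile overlapping BulletDetectionCapsule flags death, disables the collision components, ragdolls the mesh and destroys the actor after a delay.
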(event `self.ReceiveTick`
  (params (DeltaSeconds :type "Float (single-precision)"))
  (bind _returnvalue (`self.K2_GetActorLocation`))
  (bind _objectivetopursue (`self.ObjectiveToPursue`))
  (bind _returnvalue_2 (`self.K2_GetActorLocation` _objectivetopursue))
  ;[1 1 1] Estoy vivo?
  (if (`self.Alive`)
    ;[1 1 1] Tengo un objetivo?
    (if (`KismetSystemLibrary.IsValid` _objectivetopursue)
      ;[1 1 1] Calculo de la nueva posicion del zombie
      (`self.K2_SetActorLocation` (`KismetMathLibrary.VLerp` _returnvalue _returnvalue_2 0.006))
      ;[1 1 1] Calculo de la nueva rotacion del zombie
      (`self.K2_SetActorRotation` (`KismetMathLibrary.RLerp` (`KismetMathLibrary.FindLookAtRotation` _returnvalue _returnvalue_2) (`self.K2_GetActorRotation`) 0.1)))))

(event `self.Box.OnComponentBeginOverlap`
  (params (OverlappedComponent :type "PrimitiveComponent Object Reference") (OtherActor :type "Actor Object Reference") (OtherComp :type "PrimitiveComponent Object Reference") (OtherBodyIndex :type Integer) (bFromSweep :type Boolean) (SweepResult :type "HitResult Structure (by ref)"))
  ;[1 1 1] A quien me voy a comer?
  (if (== (`GameplayStatics.GetObjectClass` OtherActor) "/Game/Templates/FirstPersonBP/Blueprints/FirstPersonCharacter.FirstPersonCharacter_C")
    (set `self.ObjectiveToPursue` OtherActor)
    ;[1 1 1] Voy a correr
    (bind _aszombie_anim_bp (cast `/Game/Entities/Enemys/Zombie/ZombieAnimBP` (`SkeletalMeshComponent.GetAnimInstance` (`self.Zombie_Z_Attack`))))
    (set `/Game/Entities/Enemys/Zombie/ZombieAnimBP.IsEnemyDetected` true _aszombie_anim_bp)))

(event `self.BulletDetectionCapsule.OnComponentBeginOverlap`
  (params (OverlappedComponent :type "PrimitiveComponent Object Reference") (OtherActor :type "Actor Object Reference") (OtherComp :type "PrimitiveComponent Object Reference") (OtherBodyIndex :type Integer) (bFromSweep :type Boolean) (SweepResult :type "HitResult Structure (by ref)"))
  (bind _collisioncomponent (`self.CollisionComponent`))
  (bind _zombie_z_attack (`self.Zombie_Z_Attack`))
  ;[1 1 1] ES UNA BALA??!!!
  (cast `/Game/Templates/FirstPersonBP/Blueprints/FirstPersonProjectile` OtherActor)
  ;[1 1 1] Pos me muero
  (set `self.Alive` false)
  (bind _aszombie_anim_bp (cast `/Game/Entities/Enemys/Zombie/ZombieAnimBP` (`SkeletalMeshComponent.GetAnimInstance` (`self.Zombie_Z_Attack`))))
  (set `/Game/Entities/Enemys/Zombie/ZombieAnimBP.isDead` true _aszombie_anim_bp)
  ;[1 1 1] Bloqueo del cambio en las rotaciones y posiciones de la capsula encargada de las fisicas
  (`PrimitiveComponent.SetConstraintMode` (`self.CollisionComponent`) "SixDOF")
  ;[1 1 1] Desactivar las fisicas o colisiones
  (`PrimitiveComponent.SetSimulatePhysics` _collisioncomponent false)
  (`PrimitiveComponent.SetCollisionEnabled` _collisioncomponent "NoCollision")
  (`PrimitiveComponent.SetCollisionEnabled` (`self.Box`) "NoCollision")
  (`PrimitiveComponent.SetCollisionEnabled` (`self.BulletDetectionCapsule`) "NoCollision")
  ;[1 1 1] Soy un muñeco de trapo ahora.
  (`PrimitiveComponent.SetCollisionEnabled` _zombie_z_attack "QueryAndPhysics")
  (`PrimitiveComponent.SetSimulatePhysics` _zombie_z_attack true)
  ;[1 1 1] Espero para desaparecerme del mundo
  (`KismetSystemLibrary.Delay` 4.0)
  (`self.K2_DestroyActor`))

(fn `UserConstructionScript`)