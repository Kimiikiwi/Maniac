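; BP_DynamicWheater runs dynamic weather by switching between particle systems from the WheaterParticles array.
; BeginPlay triggers SetRandomWheater immediately and sets a timer to repeat it every WheaterDuration, looping if WheaterCycle is set.
; Each change rerolls until the index differs from the previous one, then deactivates the current system.
; The first weather activates instantly, while later ones start through a delayed SetParticleActive timer so the previous effect finishes falling.
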(event `self.ReceiveBeginPlay`
  ;[1 1 1] Evita esperar el delay que hay para el primer ciclo, para que haya clima apenas inicie el juego
  (`self.SetRandomWheater`)
  ;[1 1 1] Cambia el clima ciclicamente cada cierto tiempo
  (`KismetSystemLibrary.K2_SetTimer` null "SetRandomWheater" (`self.WheaterDuration`) (`self.WheaterCycle`)))

(fn `SetParticleActive`
  (`ActorComponent.SetActive` (`self.CurrentParticleSystem`) true false))

(fn `SetRandomWheater`
  (bind _currentparticlesystem (`self.CurrentParticleSystem`))
  ;[1 1 1] Seleccion de un clima que no sea igual al inmediatamente anterior
  (bind _output_get (set `self.TempInt` (`KismetMathLibrary.RandomInteger` (`KismetArrayLibrary.Array_Length` (`self.WheaterParticles`))) :!label _label))
  (if (!= _output_get (`self.PreviousWheater`))
    ;[1 1 1] Si hay un sistema de particulas activo apagelo, sino asigneme uno nuevo
    (bind _output_get_2 (set `self.PreviousWheater` _output_get))
    (`/Engine/EditorBlueprintResources/StandardMacros.IsValid` _currentparticlesystem
      (:`Is Valid`
        (`ActorComponent.SetActive` _currentparticlesystem false true))
      (:`Is Not Valid`
        _))
    (set `self.CurrentParticleSystem` (`Emitter.ParticleSystemComponent` (`|GetArrayItem` (`self.WheaterParticles`) _output_get_2)))
    ;[1 1 1] Como es el primer ciclo lo activa sin delay, debido a que no tiene que esperar a que termine el clima anterior, porque no hay
    (if (`self.FirstCycle`)
      (`self.SetParticleActive`)
      (set `self.FirstCycle` false)
      (else
        ;[1 1 1] Espera a que termine de caer completamente el clima anterior para activar despues el siguiente
        (`KismetSystemLibrary.K2_SetTimer` null "SetParticleActive" 15.0)))
    (else
      (goto _label))))

(fn `UserConstructionScript`)