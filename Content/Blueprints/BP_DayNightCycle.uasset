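; BP_DayNightCycle drives a day-night cycle by rotating a light actor and refreshing the sky sphere.
; Each Tick sets IsNight from whether the light's pitch exceeds a fixed threshold.
; It then adds local pitch scaled by delta time, Velocidad and FactorNoche, and calls UpdateSunDirection on SkySphere.
; FactorNoche applies regardless of IsNight, and a rotation node without that factor is left disconnected.
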(event `self.ReceiveTick`
  (params (DeltaSeconds :type "Float (single-precision)"))
  (bind _light (`self.Light`))
  (if (> (.pitch (`self.K2_GetActorRotation` _light)) 50.0)
    (set `self.bIsNight` true)
    (else
      (set `self.bIsNight` false)))
  (`self.K2_AddActorLocalRotation` _light (`KismetMathLibrary.MakeRotator` 0.0 (* (* DeltaSeconds (`self.Velocidad`)) (`self.FactorNoche`))) false false)
  (`/Engine/EngineSky/BP_Sky_Sphere.UpdateSunDirection` (`self.SkySphere`)))

(fn `UserConstructionScript`)